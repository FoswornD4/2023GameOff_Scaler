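; Repeatable interaction trigger that lets a player toggle a set of changeable objects by pressing E.
; A character overlapping the Box enables input and opens a gate; leaving disables input.
; Each press flip-flops between scaling every BP_ChangableObject target by ScaleChangeRate with changed materials and reversing it with original materials.
; Both states also swap its own material, update IsChanged and call TriggerFinished.
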(event OnComponentEndOverlap(Box)
  (params (OverlappedComponent :type Primitive%20Component%20Object%20Reference) (OtherActor :type Actor%20Object%20Reference) (OtherComp :type Primitive%20Component%20Object%20Reference) (OtherBodyIndex :type Integer))
  (Utilities|Casting|CastToCharacter OtherActor)
  (Input|DisableInput (Game|GetPlayerController 0)))

(event OnComponentBeginOverlap(Box)
  (params (OverlappedComponent :type Primitive%20Component%20Object%20Reference) (OtherActor :type Actor%20Object%20Reference) (OtherComp :type Primitive%20Component%20Object%20Reference) (OtherBodyIndex :type Integer) (bFromSweep :type Boolean) (SweepResult :type Hit%20Result%20Structure%20%28by%20ref%29))
  (Utilities|Casting|CastToCharacter OtherActor)
  (Input|EnableInput (Game|GetPlayerController 0))
  (Utilities|FlowControl|Gate true) ; enters at Open
)

(event EventBeginPlay)

(event Collision|EventActorBeginOverlap
  (params (OtherActor :type Actor%20Object%20Reference)))

(event EventTick
  (params (DeltaSeconds :type Float%20%28single-precision%29)))

(event Input|KeyboardEvents|E
  (params (Key :type Key%20Structure :default "None"))
  (:Pressed
    (Utilities|FlowControl|Gate true
      (:Exit
        (bind _isa (Utilities|FlowControl|FlipFlop)
          (:A
            ;[1 1 1] Active
            (for _array_element (Variables|Default|GetScaleChangeTarget)
              (bind _asbp_changable_object (Utilities|Casting|CastToBP_ChangableObject _array_element))
              (Transformation|SetWorldScale3D (Variables|/Script/Engine.Actor|GetRootComponent _asbp_changable_object) (* (Transformation|GetWorldScale (Variables|/Script/Engine.Actor|GetRootComponent _asbp_changable_object)) (Variables|Default|GetScaleChangeRate)))
              (Rendering|Material|SetMaterial (Variables|/Game/Blueprints/BP_ChangableObject.BP_ChangableObject_C|GetStaticMesh _asbp_changable_object) 0 (Variables|Default|GetTargetChangeMaterial)))
            (Rendering|Material|SetMaterial (Variables|Default|GetStaticMesh) 0 (Variables|Default|GetSelfChangeMaterial))
            (Variables|Default|SetIsChanged _isa)
            (Default|CallTriggerFinished))
          (:B
            ;[1 1 1] Deactive
            (for _array_element_2 (Variables|Default|GetScaleChangeTarget)
              (bind _asbp_changable_object_2 (Utilities|Casting|CastToBP_ChangableObject _array_element_2))
              (Transformation|SetWorldScale3D (Variables|/Script/Engine.Actor|GetRootComponent _asbp_changable_object_2) (/ (Transformation|GetWorldScale (Variables|/Script/Engine.Actor|GetRootComponent _asbp_changable_object_2)) (Variables|Default|GetScaleChangeRate)))
              (Rendering|Material|SetMaterial (Variables|/Game/Blueprints/BP_ChangableObject.BP_ChangableObject_C|GetStaticMesh _asbp_changable_object_2) 0 (Variables|Default|GetTargetOriginalMaterial)))
            (Rendering|Material|SetMaterial (Variables|Default|GetStaticMesh) 0 (Variables|Default|GetSelfOriginalMaterial))
            (Variables|Default|SetIsChanged _isa)
            (Default|CallTriggerFinished)))))))

(fn ConstructionScript)