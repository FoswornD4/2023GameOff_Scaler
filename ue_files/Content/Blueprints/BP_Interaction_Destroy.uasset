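; BP_Interaction_Destroy is an interaction trigger that destroys its own static mesh when E is pressed.
; Box overlap enables input and opens a gate; end overlap only disables input.
; The key press scales each BP_ChangableObject in ScaleChangeTarget by ScaleChangeRate and swaps its material to TargetMaterial.
; It then destroys the mesh, sets IsDestroyed and calls CallTriggerFinished; the Hint loop body is empty.
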(event OnComponentEndOverlap(Box)
  (params (OverlappedComponent :type Primitive%20Component%20Object%20Reference) (OtherActor :type Actor%20Object%20Reference) (OtherComp :type Primitive%20Component%20Object%20Reference) (OtherBodyIndex :type Integer))
  (Input|DisableInput (Game|GetPlayerController 0)))

(event OnComponentBeginOverlap(Box)
  (params (OverlappedComponent :type Primitive%20Component%20Object%20Reference) (OtherActor :type Actor%20Object%20Reference) (OtherComp :type Primitive%20Component%20Object%20Reference) (OtherBodyIndex :type Integer) (bFromSweep :type Boolean) (SweepResult :type Hit%20Result%20Structure%20%28by%20ref%29))
  (Input|EnableInput (Game|GetPlayerController 0))
  (Utilities|FlowControl|Gate true) ; enters at Open
)

(event EventBeginPlay)

(event Collision|EventActorBeginOverlap
  (params (OtherActor :type Actor%20Object%20Reference)))

(event EventTick
  (params (DeltaSeconds :type Float%20%28single-precision%29)))

(event Input|KeyboardEvents|E
  (params (Key :type Key%20Structure :default "None"))
  (:Pressed
    (Utilities|FlowControl|Gate true
      (:Exit
        (for _array_element (Variables|Default|GetScaleChangeTarget)
          (bind _asbp_changable_object (Utilities|Casting|CastToBP_ChangableObject _array_element))
          (Transformation|SetWorldScale3D (Variables|/Script/Engine.Actor|GetRootComponent _asbp_changable_object) (* (Transformation|GetWorldScale (Variables|/Script/Engine.Actor|GetRootComponent _asbp_changable_object)) (Variables|Default|GetScaleChangeRate)))
          (Rendering|Material|SetMaterial (Variables|/Game/Blueprints/BP_ChangableObject.BP_ChangableObject_C|GetStaticMesh _asbp_changable_object) 0 (Variables|Default|GetTargetMaterial)))
        (for _array_element_2 (Variables|Default|GetHint)
          _)
        (Components|DestroyComponent (Variables|Default|GetStaticMesh))
        (Variables|Default|SetIsDestroyed true)
        (Default|CallTriggerFinished)))))

(fn ConstructionScript)